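; Skee-ball machine that awards points when something overlaps one of its four scoring zones and shows the total on a Score widget component.
; Each zone passes its point value to AddToScore, then a shared path reads the total from ScoreKeeperGameMode and updates ScoreTextWidgetBP.
; BeginPlay resets the displayed text to zero.
; ScoreKeeperGameMode is never assigned in this graph, and an author note reports a None reference error.
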(event `self.ReceiveBeginPlay`
  (bind _asscore_text_widget_bp (cast `/Game/Blueprints/ScoreTextWidgetBP` (`WidgetComponent.GetUserWidgetObject` (`self.Score`))))
  (`/Game/Blueprints/ScoreTextWidgetBP.UpdateScore` _asscore_text_widget_bp "0"))

(event `self.40.OnComponentBeginOverlap`
  (params (OverlappedComponent :type "PrimitiveComponent Object Reference") (OtherActor :type "Actor Object Reference") (OtherComp :type "PrimitiveComponent Object Reference") (OtherBodyIndex :type Integer) (bFromSweep :type Boolean) (SweepResult :type "HitResult Structure (by ref)"))
  (`self.AddToScore` 40)
  ;[0 0 0] When reference is accessed, it is None and throws error.
  (bind _returnvalue (`DemoSkeeBallProjectGameModeBase.GetScore` (`self.ScoreKeeperGameMode`) :!label _label))
  (bind _asscore_text_widget_bp (cast `/Game/Blueprints/ScoreTextWidgetBP` (`WidgetComponent.GetUserWidgetObject` (`self.Score`))))
  (`/Game/Blueprints/ScoreTextWidgetBP.UpdateScore` _asscore_text_widget_bp (`KismetTextLibrary.Conv_IntToText` _returnvalue)))

(event `self.30.OnComponentBeginOverlap`
  (params (OverlappedComponent :type "PrimitiveComponent Object Reference") (OtherActor :type "Actor Object Reference") (OtherComp :type "PrimitiveComponent Object Reference") (OtherBodyIndex :type Integer) (bFromSweep :type Boolean) (SweepResult :type "HitResult Structure (by ref)"))
  (`self.AddToScore` 30)
  (goto _label))

(event `self.20.OnComponentBeginOverlap`
  (params (OverlappedComponent :type "PrimitiveComponent Object Reference") (OtherActor :type "Actor Object Reference") (OtherComp :type "PrimitiveComponent Object Reference") (OtherBodyIndex :type Integer) (bFromSweep :type Boolean) (SweepResult :type "HitResult Structure (by ref)"))
  (`self.AddToScore` 20)
  (goto _label))

(event `self.10.OnComponentBeginOverlap`
  (params (OverlappedComponent :type "PrimitiveComponent Object Reference") (OtherActor :type "Actor Object Reference") (OtherComp :type "PrimitiveComponent Object Reference") (OtherBodyIndex :type Integer) (bFromSweep :type Boolean) (SweepResult :type "HitResult Structure (by ref)"))
  (`self.AddToScore` 10)
  (goto _label))

(fn `UserConstructionScript`)